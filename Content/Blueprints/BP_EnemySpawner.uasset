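; BP_EnemySpawner is an actor that runs a survival countdown while spawning enemies, then triggers the player character's Victory.
; BeginPlay shows the Timer widget and starts a looping spawn timer, with its 2–5 second interval randomised once.
; Each firing spawns BP_EnemyAI at a random XY offset, or calls Victory once Minutes and Seconds run out.
; Tick uses a Delay to decrement the countdown about once per second.
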(event Custom|SpawnEnemy
  (bind _returnvalue (Transformation|GetActorLocation))
  (if (<= (Variables|Default|Getminutes) 0)
    (if (<= (Variables|Default|Getseconds) 0)
      (bind _asbp_first_person_character (Utilities|Casting|CastToBP_FirstPersonCharacter (Game|GetPlayerCharacter 0)))
      (Default|Victory _asbp_first_person_character)
      (else
        (bind _output_get (Variables|Default|SetEnemySpawnLocation (Math|Vector|MakeVector (+ (.x _returnvalue) (Math|Random|RandomFloatinRange -5e+02 5e+02)) (+ (.y _returnvalue) (Math|Random|RandomFloatinRange -5e+02 5e+02)) (.z _returnvalue)) :!label _label))
        (AI|SpawnAIFromClass "/Game/Blueprints/BP_EnemyAI.BP_EnemyAI_C" 0 _output_get "0, 0, 0" false 0)))
    (else
      (goto _label))))

(event EventBeginPlay
  (bind _returnvalue (UserInterface|CreateWidget "/Game/UI/Timer.Timer_C"))
  (UserInterface|Viewport|AddtoViewport _returnvalue 0)
  (Utilities|Time|SetTimerbyEvent (delegate Custom|SpawnEnemy) (Math|Random|RandomFloatinRange 2.0 5.0) true))

(event EventTick
  (params (DeltaSeconds :type Float%20%28single-precision%29))
  ;[1 1 1] Countdown Timer
  (Utilities|FlowControl|Delay 1.0)
  (if (<= (Variables|Default|Getminutes) 0)
    (if (not (<= (Variables|Default|Getseconds) 0))
      (Variables|Default|Setseconds (- (Variables|Default|Getseconds) 1) :!label _label)
      (if (== (Variables|Default|Getseconds) -1)
        (if (not (<= (Variables|Default|Getminutes) 0))
          (Variables|Default|Setminutes (- (Variables|Default|Getminutes) 1))
          (Variables|Default|Setseconds 59))))
    (else
      (goto _label))))

(fn ConstructionScript)