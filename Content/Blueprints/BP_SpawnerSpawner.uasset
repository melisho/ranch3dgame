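; BP_SpawnerSpawner is an actor that periodically spawns BP_EnemySpawner actors around itself during play.
; On BeginPlay it starts a looping timer whose interval is randomized once, then reused for every repeat.
; Each tick of that timer spawns a spawner at a random X/Y offset from its own location at the same height, ignoring collisions.
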(event Custom|SpawnSpawner
  (bind _returnvalue (Transformation|GetActorLocation))
  (bind _output_get (Variables|Default|SetSpawnerSpawnLocation (Math|Vector|MakeVector (+ (.x _returnvalue) (Math|Random|RandomFloatinRange -5e+02 5e+02)) (+ (.y _returnvalue) (Math|Random|RandomFloatinRange -5e+02 5e+02)) (.z _returnvalue))))
  (Game|SpawnActorfromClass "/Game/Blueprints/BP_EnemySpawner.BP_EnemySpawner_C" (Math|Conversions|ToTransform(Vector) _output_get) "AlwaysSpawn" "MultiplyWithRoot" 0 0))

(event EventBeginPlay
  (Utilities|Time|SetTimerbyEvent (delegate Custom|SpawnSpawner) (Math|Random|RandomFloatinRange 5e+01 1e+02) true))

(fn ConstructionScript)